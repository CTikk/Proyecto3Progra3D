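; Melee enemy character for the dungeon crawler that deals damage to a target within attack range.
; On BeginPlay it runs the parent logic and initializes its combat component from a data table.
; The MeleeAttack event checks that the target is valid and close enough, applies combat damage with itself as causer, and prints a debug hit message.
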(event Custom|MeleeAttack
  (params (TargetActor :type Actor%20Object%20Reference))
  (bind _self self)
  (Utilities|IsValid TargetActor
    (:Is%20Valid
      (if (<= (Math|Vector|Distance(Vector) (Transformation|GetActorLocation _self) (Transformation|GetActorLocation TargetActor)) (Variables|Default|GetAttackRange))
        (CallFunction|CombatApplyDamage TargetActor (Variables|Default|GetAttackDamage) _self)
        (Development|PrintString "Melee hit" true true "(R=1.000000,G=0.000000,B=0.006496,A=1.000000)" 2.0 "29379812793")))))

(event EventBeginPlay
  (|CallParentFunction)
  (Default|InitfromDataTable (Variables|Default|GetCombatComp)))

(event Collision|EventActorBeginOverlap
  (params (OtherActor :type Actor%20Object%20Reference))
  (|CallParentFunction OtherActor) ; This node is disabled and will not be called.\nDrag off pins to build functionality.
)

(event EventTick
  (params (DeltaSeconds :type Float%20%28single-precision%29))
  (|CallParentFunction DeltaSeconds) ; This node is disabled and will not be called.\nDrag off pins to build functionality.
)

(fn ConstructionScript
  (|CallParentFunction))