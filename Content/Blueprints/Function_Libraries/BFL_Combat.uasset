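; Blueprint function library of shared combat helpers for attacking and damaging actors.
; CombatAttack reads BaseDamage from the attacker's AC_CombatStats component and passes it to CombatApplyDamage with the target.
; CombatApplyDamage calls the engine's ApplyDamage, then plays the damaged actor's HitVFX and HitSFX at its location, both gated only on HitVFX being set.
; GetCombatComponent provides the component lookup for both functions.
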(fn GetCombatComponent
  (params (TargetActor :type Actor%20Object%20Reference))
  (Utilities|IsValid TargetActor
    (:Is%20Valid
      (return (Actor|GetComponentbyClass TargetActor "/Game/Blueprints/Components/AC_CombatStats.AC_CombatStats_C")))))

(fn CombatApplyDamage
  (params (DamagedActor :type Actor%20Object%20Reference) (DamageAmount :type Float%20%28double-precision%29) (DamageCauser :type Actor%20Object%20Reference))
  (bind _returnvalue (Transformation|GetActorLocation DamagedActor))
  (Game|Damage|ApplyDamage DamagedActor DamageAmount 0 DamageCauser)
  (bind _combatcomponent (CallFunction|GetCombatComponent DamagedActor))
  (if (!= (Variables|/Game/Blueprints/Components/AC_CombatStats.AC_CombatStats_C|GetHitVFX _combatcomponent) 0)
    (Niagara|SpawnSystematLocation 0 (Variables|/Game/Blueprints/Components/AC_CombatStats.AC_CombatStats_C|GetHitVFX _combatcomponent) _returnvalue)
    (Audio|PlaySoundatLocation 0 (Variables|/Game/Blueprints/Components/AC_CombatStats.AC_CombatStats_C|GetHitSFX _combatcomponent) _returnvalue "0, 0, 0" 1.0 1.0 0.0 0 0 0 0)))

(fn CombatAttack
  (params (Attacker :type Actor%20Object%20Reference) (Target :type Actor%20Object%20Reference))
  (bind _combatcomponent (CallFunction|GetCombatComponent Attacker))
  (if (!= _combatcomponent 0)
    (CallFunction|CombatApplyDamage Target (Variables|/Game/Blueprints/Components/AC_CombatStats.AC_CombatStats_C|GetBaseDamage _combatcomponent) Attacker)))