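; Base trap actor that starts offset from its placed position and, when activated, rises to damage the player.
; BeginPlay derives the hidden location from RiseHeight; ActivateTrap lerps to the surface via timeline and sets a timer for LowerTrap, which reverses the motion.
; DamageZone collision is enabled only while active, applying CombatApplyDamage to an overlapping BP_ThirdPersonCharacter.
; DeactivateTrap disables damage without moving the trap.
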(event OnComponentBeginOverlap(DamageZone)
  (params (OverlappedComponent :type Primitive%20Component%20Object%20Reference) (OtherActor :type Actor%20Object%20Reference) (OtherComp :type Primitive%20Component%20Object%20Reference) (OtherBodyIndex :type Integer) (bFromSweep :type Boolean) (SweepResult :type Hit%20Result%20Structure%20%28by%20ref%29))
  (Utilities|Casting|CastToBP_ThirdPersonCharacter OtherActor)
  (if (Variables|Default|GetIsActive)
    (CallFunction|CombatApplyDamage OtherActor (Variables|Default|GetDamage) self)
    (Development|PrintString "Trap hit Player" true true "(R=0.000000,G=1.000000,B=0.109664,A=1.000000)" 2.0 "298173")))

(event Custom|RiseTrap
  (Variables|Default|SetIsActive true)
  (Collision|SetCollisionEnabled (Variables|Default|GetDamageZone) "QueryOnly")
  (bind _alpha (Timeline|Timeline Play)
    (:Update
      (Transformation|SetActorLocation (Math|Vector|Lerp(Vector) (Variables|Default|GetHiddenLocation) (Variables|Default|GetSurfaceLocation) _alpha) false false)
      (Development|PrintString "Trap Activated" true true "(R=0.233716,G=1.000000,B=0.147532,A=1.000000)" 2.0 "121982"))))

(event Custom|LowerTrap
  (Variables|Default|SetIsActive false)
  (Collision|SetCollisionEnabled (Variables|Default|GetDamageZone) "NoCollision")
  (bind _alpha (Timeline|Timeline_0 ReverseFromEnd)
    (:Update
      (Transformation|SetActorLocation (Math|Vector|Lerp(Vector) (Variables|Default|GetHiddenLocation) (Variables|Default|GetSurfaceLocation) _alpha) false false))))

(event EventBeginPlay
  (bind _output_get (Variables|Default|SetSurfaceLocation (Transformation|GetActorLocation self)))
  (bind _result (Math|Float|NegateFloat (Variables|Default|GetRiseHeight))
    (:%20%20
      (bind _output_get_2 (Variables|Default|SetHiddenLocation (+ _output_get (Math|Vector|MakeVector 0.0 0.0 _result))))
      (Transformation|SetActorLocation _output_get_2 false false))))

(event Collision|EventActorBeginOverlap
  (params (OtherActor :type Actor%20Object%20Reference)))

(event EventTick
  (params (DeltaSeconds :type Float%20%28single-precision%29)))

(event EventActivateTrap
  (params (InstigatorActor :type Actor%20Object%20Reference))
  (if (not (Variables|Default|GetIsActive))
    (Variables|Default|SetIsActive true)
    (CallFunction|RiseTrap)
    (Utilities|Time|SetTimerbyEvent (delegate Custom|LowerTrap) (Variables|Default|GetActiveDuration))))

(fn ConstructionScript)

(fn DeactivateTrap
  (Variables|Default|SetIsActive false)
  (Collision|SetCollisionEnabled (Variables|Default|GetDamageZone) "NoCollision")
  (Development|PrintString "Trap deactivated" true true "(R=1.000000,G=0.419256,B=0.000000,A=1.000000)" 2.0 "3972193"))