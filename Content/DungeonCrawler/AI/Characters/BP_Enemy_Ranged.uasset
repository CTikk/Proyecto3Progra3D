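; Ranged enemy character that patrols via an AI Blackboard and shoots projectiles at targets.
; On BeginPlay it casts its controller to BP_RangedAIController and seeds the Blackboard with a home location from the controller's location, plus the first patrol point and index when patrol points exist.
; FireAtTarget turns the actor toward the given target and spawns its configurable projectile class aimed at that target's position.
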(event Custom|FireAtTarget
  (params (TargetActor :type Actor%20Object%20Reference))
  (bind _returnvalue (Transformation|GetActorLocation))
  (bind _returnvalue_2 (Transformation|GetActorLocation TargetActor))
  (bind _returnvalue_3 (Math|Rotator|FindLookatRotation _returnvalue _returnvalue_2))
  (Transformation|SetActorRotation _returnvalue_3)
  (if (Utilities|IsValid TargetActor)
    (Variables|Default|SetTargetLocation (Transformation|GetActorLocation TargetActor))
    (Game|SpawnActorfromClass (Variables|Default|GetProjectileClass) (Math|Transform|MakeTransform (Transformation|GetActorLocation self) _returnvalue_3) "AdjustIfPossibleButAlwaysSpawn" "MultiplyWithRoot" 0 0)))

(event EventBeginPlay
  (bind _returnvalue (Pawn|GetController))
  (bind _patrolpoints (Variables|Default|GetPatrolPoints))
  (|CallParentFunction)
  (bind _asbp_ranged_aicontroller (Utilities|Casting|CastToBP_RangedAIController _returnvalue))
  (AI|Components|Blackboard|SetValueasVector (AI|GetBlackboard _asbp_ranged_aicontroller) (Variables|Default|GetHomeLocation) (Transformation|GetActorLocation _returnvalue))
  (if (> (Utilities|Array|Length _patrolpoints) 0)
    (Class|BlackboardComponent|SetValueasInt (AI|GetBlackboard _asbp_ranged_aicontroller) (Variables|Default|GetCurrentPatrolIndex))
    (AI|Components|Blackboard|SetValueasVector (AI|GetBlackboard _asbp_ranged_aicontroller) (Variables|Default|GetPatrolLocation) (Transformation|GetActorLocation (Utilities|Array|Get(acopy) _patrolpoints)))))

(event Collision|EventActorBeginOverlap
  (params (OtherActor :type Actor%20Object%20Reference))
  (|CallParentFunction OtherActor) ; This node is disabled and will not be called.\nDrag off pins to build functionality.
)

(event EventTick
  (params (DeltaSeconds :type Float%20%28single-precision%29))
  (|CallParentFunction DeltaSeconds) ; This node is disabled and will not be called.\nDrag off pins to build functionality.
)

(fn ConstructionScript
  (|CallParentFunction))