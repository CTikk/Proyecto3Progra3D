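; Base enemy character for the dungeon crawler that sets health and walk speed on spawn and exposes its team.
; AnyDamage passes hits to CombatComp and calls Die when that returns true, while a separate ReceiveDamage function tracks CurrentHealth and IsDead itself.
; Die stops the AI controller, disables capsule collision, ragdolls the mesh, detaches the controller and sets a short life span for cleanup.
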(event EventBeginPlay
  (Variables|Default|SetCurrentHealth (Variables|Default|GetMaxHealth))
  (Variables|/Script/Engine.CharacterMovementComponent|SetMaxWalkSpeed (Variables|Character|GetCharacterMovement) (Variables|Default|GetWalkSpeed)))

(event Collision|EventActorBeginOverlap
  (params (OtherActor :type Actor%20Object%20Reference)))

(event EventTick
  (params (DeltaSeconds :type Float%20%28single-precision%29)))

(event Game|Damage|EventAnyDamage
  (params (Damage :type Float%20%28single-precision%29) (DamageType :type Damage%20Type%20Object%20Reference) (InstigatedBy :type Controller%20Object%20Reference) (DamageCauser :type Actor%20Object%20Reference))
  (bind _died (Default|ApplyDamagetoSelf (Variables|Default|GetCombatComp) Damage DamageCauser))
  (Development|PrintString "Applied Dmg to self enemy" true true "(R=1.000000,G=0.000000,B=0.032783,A=1.000000)" 2.0 "298173")
  (if _died
    (CallFunction|Die)))

(fn ConstructionScript)

(fn ReceiveDamage
  (params (DamageAmount :type Float%20%28double-precision%29) (DamageCauser :type Actor%20Object%20Reference))
  (Development|PrintString "in enemy receive dmg")
  (if (not (Variables|Default|GetIsDead))
    (bind _output_get (Variables|Default|SetCurrentHealth (- (Variables|Default|GetCurrentHealth) DamageAmount)))
    (if (<= _output_get 0.0)
      (Variables|Default|SetIsDead true)
      (CallFunction|Die)
      (else
        (Development|PrintString (Utilities|String|ToString(Float) _output_get) true true "(R=1.000000,G=0.000000,B=0.037934,A=1.000000)")))))

(fn Die
  (bind _capsulecomponent (Variables|Collision|GetCapsuleComponent))
  (bind _mesh (Variables|Character|GetMesh))
  (bind _asaicontroller (Utilities|Casting|CastToAIController (Pawn|GetController)))
  (AI|Navigation|StopMovement _asaicontroller)
  (Collision|SetCollisionEnabled _capsulecomponent "NoCollision")
  (Collision|SetCollisionResponsetoAllChannels _capsulecomponent "ECR_Ignore")
  (Collision|SetCollisionProfileName (Variables|Character|GetMesh) "Ragdoll" true :!class /Script/Engine.PrimitiveComponent)
  (Physics|SetSimulatePhysics _mesh true)
  (Physics|SetEnableGravity _mesh true)
  (Class|SkeletalMeshComponent|SetAllBodiesBelowSimulatePhysics _mesh (LocalVariables|GetPelvis) true true)
  (Class|Pawn|DetachfromControllerPendingDestroy)
  (Actor|SetLifeSpan 5.0)
  (Development|PrintString "Enemy dead" true true "(R=1.000000,G=0.000000,B=0.240963,A=1.000000)" 2.0 "1234455"))

(fn GetTeam
  (bind _team (Variables|Default|GetTeam))
  (return (Utilities|Name|EnumtoName _team) _team))