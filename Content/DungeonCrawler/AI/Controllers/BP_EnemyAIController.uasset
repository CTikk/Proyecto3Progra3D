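; BP_EnemyAIController is the AI controller for dungeon crawler enemies, starting their behavior tree on BeginPlay.
; When AI perception successfully senses the player character, it writes that actor to the TargetActor blackboard key and prints a debug message.
; If the controlled pawn is a BP_Enemy_Scout, it also has the scout alert nearby enemies to the player.
; Lost sightings are ignored, so this controller never clears the target.
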(event OnTargetPerceptionUpdated(AIPerception)
  (params (Actor :type Actor%20Object%20Reference) (Stimulus :type AI%20Stimulus%20Structure))
  (if (.bSuccessfullySensed (Utilities|Struct|BreakAIStimulus Stimulus))
    (Utilities|Casting|CastToBP_ThirdPersonCharacter Actor)
    (AI|Components|Blackboard|SetValueasObject (Variables|Default|GetBlackboard) (Variables|Default|GetTargetActor) Actor)
    (Development|PrintString "Player Seen" true true "(R=1.000000,G=0.000000,B=0.931964,A=1.000000)" 2.0 "8497398")
    (bind _asbp_enemy_scout (Utilities|Casting|CastToBP_Enemy_Scout (Pawn|GetControlledPawn)))
    (Default|SendAlerttoNearbyEnemies _asbp_enemy_scout Actor)))

(event EventBeginPlay
  (AI|RunBehaviorTree (Variables|Default|GetEnemyBehaviorTree)))

(event EventTick
  (params (DeltaSeconds :type Float%20%28single-precision%29)))

(fn ConstructionScript)