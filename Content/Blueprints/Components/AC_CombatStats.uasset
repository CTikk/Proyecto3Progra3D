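; AC_CombatStats is a combat stats component that tracks health and death for its owner.
; InitFromDataTable copies max health, damage, attack rate and hit VFX/SFX from a named StatsTable row, leaving CurrentHealth untouched.
; ApplyDamageToSelf subtracts damage while alive, truncates health to a whole number clamped to MaxHealth, and sets and returns IsDead, ignoring DamageCauser.
; Its event graph is empty, so both functions rely on external callers.
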(event EventBeginPlay)

(event EventTick
  (params (DeltaSeconds :type Float%20%28single-precision%29)))

(fn InitfromDataTable
  (bind _statstable (Variables|Default|GetStatsTable))
  (bind _rowname (Variables|Default|GetRowName))
  (if (and (!= _statstable 0) (!= _rowname ""))
    (bind _returnvalue (Utilities|GetDataTableRow _statstable _rowname)
      (:then
        (Variables|Default|SetMaxHealth (.MaxHealth (Utilities|Struct|BreakST_CombatStats _returnvalue)))
        (Variables|Default|SetBaseDamage (.BaseDamage (Utilities|Struct|BreakST_CombatStats _returnvalue)))
        (Variables|Default|SetAttackRate (.AttackRate (Utilities|Struct|BreakST_CombatStats _returnvalue)))
        (Variables|Default|SetHitVFX (.HitVFX (Utilities|Struct|BreakST_CombatStats _returnvalue)))
        (Variables|Default|SetHitSFX (.HitSFX (Utilities|Struct|BreakST_CombatStats _returnvalue)))))))

(fn ApplyDamagetoSelf
  (params (DamageAmount :type Float%20%28double-precision%29) (DamageCauser :type Actor%20Object%20Reference))
  (if (Variables|Default|GetIsDead)
    _
    (else
      (bind _output_get (Variables|Default|SetCurrentHealth (Math|Conversions|ToFloat(Integer) (Math|Integer|Clamp(Integer) (Math|Float|Truncate (- (Variables|Default|GetCurrentHealth) DamageAmount)) 0 (Math|Float|Truncate (Variables|Default|GetMaxHealth))))))
      (if (> _output_get 0.0)
        (Variables|Default|SetIsDead false)
        (else
          (Variables|Default|SetIsDead true)))))
  (return (Variables|Default|GetIsDead)))